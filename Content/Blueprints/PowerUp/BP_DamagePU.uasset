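; BP_DamagePU is a damage power-up pickup that permanently raises the Damage stat of the player character that touches it.
; On box overlap it casts the other actor to the Aurora, Khaimera or Terra player character in turn and adds a flat bonus.
; It then swaps its Niagara effect, disables box collision to prevent repeat pickups and destroys itself after a short delay.
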(event OnComponentBeginOverlap(Box)
  (params (OverlappedComponent :type Primitive%20Component%20Object%20Reference) (OtherActor :type Actor%20Object%20Reference) (OtherComp :type Primitive%20Component%20Object%20Reference) (OtherBodyIndex :type Integer) (bFromSweep :type Boolean) (SweepResult :type Hit%20Result%20Structure%20%28by%20ref%29))
  (bind _asaurora_player_character (Utilities|Casting|CastToAuroraPlayerCharacter OtherActor)
    (:then
      (Variables|/Game/Blueprints/Characters/Aurora/AuroraPlayerCharacter.AuroraPlayerCharacter_C|SetDamage _asaurora_player_character (+ (Variables|/Game/Blueprints/Characters/Aurora/AuroraPlayerCharacter.AuroraPlayerCharacter_C|GetDamage _asaurora_player_character) 5.0)))
    (:CastFailed
      (bind _askhaimera_player_character (Utilities|Casting|CastToKhaimeraPlayerCharacter OtherActor)
        (:then
          (Variables|/Game/Blueprints/Characters/Khaimera/KhaimeraPlayerCharacter.KhaimeraPlayerCharacter_C|SetDamage _askhaimera_player_character (+ (Variables|/Game/Blueprints/Characters/Khaimera/KhaimeraPlayerCharacter.KhaimeraPlayerCharacter_C|GetDamage _askhaimera_player_character) 5.0)))
        (:CastFailed
          (bind _asterra_player_character (Utilities|Casting|CastToTerraPlayerCharacter OtherActor))
          (Variables|/Game/Blueprints/Characters/Terra/TerraPlayerCharacter.TerraPlayerCharacter_C|SetDamage _asterra_player_character (+ (Variables|/Game/Blueprints/Characters/Terra/TerraPlayerCharacter.TerraPlayerCharacter_C|GetDamage _asterra_player_character) 5.0))))))
  (Class|NiagaraComponent|SetAsset (Variables|NiagaraActor|GetNiagaraComponent) "/Game/sA_PickupSet_1/Fx/NiagaraSystems/NS_Energy_2.NS_Energy_2" true)
  (CallFunction|DisableCollision)
  (Utilities|FlowControl|Delay 3.0)
  (Actor|DestroyActor))

(event Custom|DisableCollision
  (Collision|SetCollisionEnabled (Variables|Default|GetBox) "NoCollision"))

(event Custom|EnableCollision
  (Collision|SetCollisionEnabled (Variables|Default|GetBox) "QueryAndPhysics"))

(event EventBeginPlay
  (CallFunction|EnableCollision))

(fn ConstructionScript)