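; BP_HealthPU is a health power-up that adds a fixed amount of health to the player character that overlaps its box.
; The overlap event casts in turn to the Aurora, Khaimera and Terra player characters and adds to Health directly, with no clamp.
; All three branches then switch the Niagara component to a healing effect and destroy the actor after a short delay.
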(event OnComponentBeginOverlap(Box)
  (params (OverlappedComponent :type Primitive%20Component%20Object%20Reference) (OtherActor :type Actor%20Object%20Reference) (OtherComp :type Primitive%20Component%20Object%20Reference) (OtherBodyIndex :type Integer) (bFromSweep :type Boolean) (SweepResult :type Hit%20Result%20Structure%20%28by%20ref%29))
  (bind _asaurora_player_character (Utilities|Casting|CastToAuroraPlayerCharacter OtherActor)
    (:then
      (Variables|/Game/Blueprints/Characters/Aurora/AuroraPlayerCharacter.AuroraPlayerCharacter_C|SetHealth _asaurora_player_character (+ (Variables|/Game/Blueprints/Characters/Aurora/AuroraPlayerCharacter.AuroraPlayerCharacter_C|GetHealth _asaurora_player_character) 5e+01)))
    (:CastFailed
      (bind _askhaimera_player_character (Utilities|Casting|CastToKhaimeraPlayerCharacter OtherActor)
        (:then
          (Variables|/Game/Blueprints/Characters/Khaimera/KhaimeraPlayerCharacter.KhaimeraPlayerCharacter_C|SetHealth _askhaimera_player_character (+ (Variables|/Game/Blueprints/Characters/Khaimera/KhaimeraPlayerCharacter.KhaimeraPlayerCharacter_C|GetHealth _askhaimera_player_character) 5e+01)))
        (:CastFailed
          (bind _asterra_player_character (Utilities|Casting|CastToTerraPlayerCharacter OtherActor))
          (Variables|/Game/Blueprints/Characters/Terra/TerraPlayerCharacter.TerraPlayerCharacter_C|SetHealth _asterra_player_character (+ (Variables|/Game/Blueprints/Characters/Terra/TerraPlayerCharacter.TerraPlayerCharacter_C|GetHealth _asterra_player_character) 5e+01))))))
  (Class|NiagaraComponent|SetAsset (Variables|NiagaraActor|GetNiagaraComponent) "/Game/sA_PickupSet_1/Fx/NiagaraSystems/NS_Healing_1.NS_Healing_1" true)
  (Utilities|FlowControl|Delay 3.0)
  (Actor|DestroyActor))

(fn ConstructionScript)